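; BP_Baker is an AI character that alternates between looking and not looking, showing a spotlight while looking, and damages the hit actor on a kill.
; BeginPlay binds look, not-look, idle and kill events; timed delays feed two alternating gates that switch the AI state.
; Idle hides the light and sets a Test flag that blocks those switches, while a kill applies damage then returns to looking after a delay.
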(event `self.ReceiveBeginPlay`
  (add `self.OnLook` (delegate `OnLook_Event`))
  (add `self.OnKill` (delegate `OnKill_Event`))
  (add `self.OnNotLook` (delegate `OnNotLook_Event`))
  (add `self.OnIdle` (delegate `OnIdle_Event`)))

(event `OnLook_Event`
  ;[1 1 1] OnLook
  (set `self.Test` false)
  (`|ExecutionSequence`
    (:`then_0`
      (`|ExecutionSequence`
        (:`then_0`
          (goto _label_2 :!via `Close`))
        (:`then_1`
          (goto _label :!via `Open`))))
    (:`then_1`
      (`KismetSystemLibrary.Delay` (`self.LookTime`))
      (`/Engine/EditorBlueprintResources/StandardMacros.Gate` false :!label _label
        (:`Exit`
          (if (not (`self.Test`))
            (`self.UpdateBakerAIState` "ENotLooking")))))
    (:`then_2`
      (`SceneComponent.SetVisibility` (`self.SpotLight1`) true false))))

(event `OnKill_Event`
  ;[1 1 1] OnKill
  (`|ExecutionSequence`
    (:`then_1`
      (`GameplayStatics.ApplyDamage` (`self.HitActor`) 1.0)
      (`KismetSystemLibrary.Delay` (`self.KillDelay`))
      (`self.UpdateBakerAIState` "ELooking"))))

(event `OnNotLook_Event`
  ;[1 1 1] OnNotLook
  (set `self.Test` false)
  (`|ExecutionSequence`
    (:`then_0`
      (`|ExecutionSequence`
        (:`then_0`
          (goto _label_2 :!via `Open`))
        (:`then_1`
          (goto _label :!via `Close`))))
    (:`then_1`
      (`KismetSystemLibrary.Delay` (`self.LookAwayTime`))
      (`/Engine/EditorBlueprintResources/StandardMacros.Gate` false :!label _label_2
        (:`Exit`
          (if (not (`self.Test`))
            (`self.UpdateBakerAIState` "ELooking")))))
    (:`then_2`
      (`SceneComponent.SetVisibility` (`self.SpotLight1`) false false))))

(event `OnIdle_Event`
  (set `self.Test` true)
  (`SceneComponent.SetVisibility` (`self.SpotLight1`) false false)
  (`KismetSystemLibrary.Delay` (`self.LookAwayTime`)))

(fn `DeathFunction`
  (returns (HitActor :type "Actor Object Reference"))
  (bind _hitactor (`self.HitActor`))
  (`self.DisableInput` _hitactor null)
  (return _hitactor))

(fn `UserConstructionScript`)