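; BP_NPC3 is an NPC that shows a line-by-line dialogue and triggers a one-time cutscene when the conversation ends.
; Each Talk event advances an index into Dialogue1 and writes that line to a lazily created WB_DialogueWidget1.
; Past the last line it removes the widget and opens the Shreks_beastly_roar media source.
; A DoOnce then plays a level sequence, disabling BP_MainCharacter's input for the sequence's duration.
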(event `self.Talk`
  (bind _sequenceplayer (`LevelSequenceActor.SequencePlayer` (`self.PlaySequence`)))
  (`/Engine/EditorBlueprintResources/StandardMacros.IncrementInt` (`self.talkIndex`)
    (:`  `
      (if (< (`self.talkIndex`) (`KismetArrayLibrary.Array_Length` (`self.dialogue1`)))
        (`self.UI`
          (:`then`
            _)
          (:`else`
            (bind _returnvalue (`|CreateWidget` "/Game/Blueprints/DialogueWidget/WB_DialogueWidget1.WB_DialogueWidget1_C" (`GameplayStatics.GetPlayerController` 0)))
            (bind _output_get (set `self.UI` _returnvalue))
            (`UserWidget.AddToViewport` _output_get 0)))
        (`TextBlock.SetText` (`/Game/Blueprints/DialogueWidget/WB_DialogueWidget1.TalkText` (`self.UI`)) (`KismetTextLibrary.Conv_StringToText` (`|GetArrayItem` (`self.dialogue1`) (`self.talkIndex`))))
        (else
          (`Widget.RemoveFromParent` (`self.UI`))
          (`MediaPlayer.OpenSource` (`self.mediaPlayer`) "/Game/Blueprints/Level/Cutscenes/Shreks_beastly_roar.Shreks_beastly_roar")
          (`/Engine/EditorBlueprintResources/StandardMacros.DoOnce` false
            (:`Completed`
              (bind _asbp_main_character (cast `/Game/Blueprints/Player/BP_MainCharacter` (`GameplayStatics.GetPlayerCharacter` 0)))
              (`self.DisableInput` _asbp_main_character null)
              (`MovieSceneSequencePlayer.Play` _sequenceplayer)
              (`KismetSystemLibrary.Delay` (`TimeManagementBlueprintLibrary.Conv_QualifiedFrameTimeToSeconds` (`MovieSceneSequencePlayer.GetDuration` _sequenceplayer)))
              (`self.EnableInput` _asbp_main_character null))))))))

(fn `UserConstructionScript`)