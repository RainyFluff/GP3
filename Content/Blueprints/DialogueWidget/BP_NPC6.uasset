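; BP_NPC6 is an NPC that shows a line-by-line dialogue through a WB_DialogueWidget1 widget.
; Each Talk call advances an index into the Dialogue1 array, creating the widget once, updating its text and adding it to the viewport.
; Running out of lines, or the main character leaving TriggerZone, resets the index and removes the widget.
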(event `self.Talk`
  (`/Engine/EditorBlueprintResources/StandardMacros.IncrementInt` (`self.talkIndex`)
    (:`  `
      (if (< (`self.talkIndex`) (`KismetArrayLibrary.Array_Length` (`self.dialogue1`)))
        (`self.UI`
          (:`then`
            _)
          (:`else`
            (bind _returnvalue (`|CreateWidget` "/Game/Blueprints/DialogueWidget/WB_DialogueWidget1.WB_DialogueWidget1_C" (`GameplayStatics.GetPlayerController` 0)))
            (bind _output_get (set `self.UI` _returnvalue))
            (`UserWidget.AddToViewport` _output_get 0)))
        (`TextBlock.SetText` (`/Game/Blueprints/DialogueWidget/WB_DialogueWidget1.TalkText` (`self.UI`)) (`KismetTextLibrary.Conv_StringToText` (`|GetArrayItem` (`self.dialogue1`) (`self.talkIndex`))))
        (`UserWidget.AddToViewport` (`self.UI`) 0)
        (else
          (set `self.talkIndex` -1)
          (`Widget.RemoveFromParent` (`self.UI`)))))))

(event `self.ReceiveTick`
  (params (DeltaSeconds :type "Float (single-precision)")))

(event `self.Trigger zone.OnComponentEndOverlap`
  (params (OverlappedComponent :type "PrimitiveComponent Object Reference") (OtherActor :type "Actor Object Reference") (OtherComp :type "PrimitiveComponent Object Reference") (OtherBodyIndex :type Integer))
  (cast `/Game/Blueprints/Player/BP_MainCharacter` OtherActor)
  (set `self.talkIndex` -1)
  (`Widget.RemoveFromParent` (`self.UI`)))

(fn `UserConstructionScript`)