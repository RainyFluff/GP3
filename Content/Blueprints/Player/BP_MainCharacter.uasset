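; Player character that handles pausing, death, dialogue, ledge climbing and size-changing beans.
; Interact scans overlapping actors, either talking through BPI_Dialogue or eating a growing or shrinking bean whose size state drives a timeline scale lerp.
; Any damage ragdolls the mesh, disables input and shows a paused failure screen after a delay; a debug key triggers it.
; Ledge mantle moves the actor forward and up along a timeline while IsClimbingUp is set.
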(event Input|EnhancedActionEvents|EnhancedInputActionIA_Pause
  (params (ActionValue :type Boolean) (ElapsedSeconds :type Float%20%28double-precision%29) (TriggeredSeconds :type Float%20%28double-precision%29) (InputAction :type Input%20Action%20Object%20Reference :default "/Game/ThirdPerson/Input/Actions/IA_Pause.IA_Pause"))
  (bind _returnvalue (Game|GetPlayerController 0))
  ;[1 1 1] Pause Menu?
  (bind _returnvalue_2 (UserInterface|CreateWidget "/Game/UI/PauseMenu.PauseMenu_C"))
  (UserInterface|Viewport|AddtoViewport _returnvalue_2 0)
  (Variables|/Script/Engine.PlayerController|SetbShowMouseCursor _returnvalue true)
  (Input|SetInputModeUIOnly _returnvalue 0 "DoNotLock" false)
  (Game|SetGamePaused true))

(event Input|EnhancedActionEvents|EnhancedInputActionIA_Interact
  (params (ActionValue :type Boolean) (ElapsedSeconds :type Float%20%28double-precision%29) (TriggeredSeconds :type Float%20%28double-precision%29) (InputAction :type Input%20Action%20Object%20Reference :default "/Game/ThirdPerson/Input/Actions/IA_Interact.IA_Interact"))
  (bind _self self)
  (bind _self_2 self)
  (:Started
    (bind _array_element (Utilities|Array|ForEachLoopwithBreak (Collision|GetOverlappingActors "/Script/Engine.Actor" :!class /Script/Engine.Actor) :!label _label)
      (:LoopBody
        (if (Utilities|DoesObjectImplementInterface _array_element "/Game/Blueprints/DialogueWidget/BPI_Dialogue.BPI_Dialogue_C")
          (Class|BPIDialogue|Talk(Message) _array_element)
          (goto _label Break)
          (elif (not (Variables|Default|GetIsEating))
            (Utilities|FlowControl|Sequence
              (:then_0
                (bind _asbp_growing_bean (Utilities|Casting|CastToBP_GrowingBean _array_element))
                (Utilities|FlowControl|Sequence
                  (:then_0
                    (goto _label Break))
                  (:then_1
                    (bind _output_get (Variables|/Script/MAL_WAR_GP3_Team04.MagicBean|SetCharacter _asbp_growing_bean _self_2))
                    (bind _output_get_2 (Variables|/Script/MAL_WAR_GP3_Team04.MagicBean|SetCharaSize _asbp_growing_bean (Transformation|GetActorScale3D _output_get)))
                    (Variables|Default|SetCamLengthChanged (Variables|/Script/MAL_WAR_GP3_Team04.MagicBean|GetChangedLengthCam _asbp_growing_bean))
                    (bind _returnvalue (Class|MagicBean|UpdateSizeStates _asbp_growing_bean _self_2 "Big"))
                    (bind _growth (Timeline|GrowthTimeline PlayFromStart)
                      (:Update
                        (Transformation|SetActorScale3D _output_get (Math|Vector|Lerp(Vector) _output_get_2 _returnvalue _growth))
                        (Variables|Default|SetIsEating true)
                        (Utilities|FlowControl|Delay 1.0)
                        (Variables|Default|SetIsEating false))))))
              (:then_1
                (bind _asbp_shrinking_bean (Utilities|Casting|CastToBP_ShrinkingBean _array_element))
                (Utilities|FlowControl|Sequence
                  (:then_0
                    (goto _label Break))
                  (:then_1
                    (bind _output_get_3 (Variables|/Script/MAL_WAR_GP3_Team04.MagicBean|SetCharacter _asbp_shrinking_bean _self))
                    (bind _output_get_4 (Variables|/Script/MAL_WAR_GP3_Team04.MagicBean|SetCharaSize _asbp_shrinking_bean (Transformation|GetActorScale3D _output_get_3)))
                    (Variables|Default|SetCamLengthChanged (Variables|/Script/MAL_WAR_GP3_Team04.MagicBean|GetChangedLengthCam _asbp_shrinking_bean))
                    (bind _returnvalue_2 (Class|MagicBean|UpdateSizeStates _asbp_shrinking_bean _self "Small"))
                    (bind _growth_2 (Timeline|Timeline PlayFromStart)
                      (:Update
                        (Transformation|SetActorScale3D _output_get_3 (Math|Vector|Lerp(Vector) _output_get_4 _returnvalue_2 _growth_2))
                        (Variables|Default|SetIsEating true)
                        (Utilities|FlowControl|Delay 1.0)
                        (Variables|Default|SetIsEating false)))))))))))))

(event Input|EnhancedActionEvents|EnhancedInputActionIA_LedgeMantle
  (params (ActionValue :type Boolean) (ElapsedSeconds :type Float%20%28double-precision%29) (TriggeredSeconds :type Float%20%28double-precision%29) (InputAction :type Input%20Action%20Object%20Reference :default "/Game/ThirdPerson/Input/Actions/IA_LedgeMantle.IA_LedgeMantle"))
  (bind _returnvalue (Transformation|GetActorLocation))
  ;[1 1 1] Climbing animation/TimeLine
  (if (Variables|Default|GetisClimbingUp)
    (bind (_direction _climbforward _climbupward) (Timeline|ClimbForward PlayFromStart)
      (:Update
        (Transformation|SetActorLocation (Math|Vector|MakeVector (.x (+ (* _climbforward (Transformation|GetActorForwardVector)) _returnvalue)) (.y (+ (* _climbforward (Transformation|GetActorForwardVector)) _returnvalue)) (.z (+ _returnvalue _climbupward))) false false)))))

(event EventBeginPlay
  ;[1 1 1] Enhanced Input System?
  (bind _asplayer_controller (Utilities|Casting|CastToPlayerController (Pawn|GetController)))
  (Utilities|IsValid (PlayerController|LocalPlayerSubsystems|GetEnhancedInputLocalPlayerSubsystem _asplayer_controller)
    (:Is%20Valid
      (Input|AddMappingContext (PlayerController|LocalPlayerSubsystems|GetEnhancedInputLocalPlayerSubsystem _asplayer_controller) "/Game/ThirdPerson/Input/IMC_Default.IMC_Default" 0 "(bIgnoreAllPressedKeysUntilRelease=True,bForceImmediately=False,bNotifyUserSettings=False)"))))

(event Game|Damage|EventAnyDamage
  (params (Damage :type Float%20%28single-precision%29) (DamageType :type Damage%20Type%20Object%20Reference) (InstigatedBy :type Controller%20Object%20Reference) (DamageCauser :type Actor%20Object%20Reference))
  (bind _returnvalue (Game|GetPlayerController 0))
  ;[1 1 1] Pause Game when player dies?
  (Physics|SetSimulatePhysics (Variables|Character|GetMesh) true)
  (Pawn|Components|CharacterMovement|DisableMovement (Variables|Character|GetCharacterMovement))
  (Input|DisableInput 0)
  (Utilities|FlowControl|Delay 2.0)
  (bind _returnvalue_2 (UserInterface|CreateWidget "/Game/UI/FailureScreen.FailureScreen_C"))
  (UserInterface|Viewport|AddtoViewport _returnvalue_2 0)
  (Variables|/Script/Engine.PlayerController|SetbShowMouseCursor _returnvalue true)
  (Input|SetInputModeUIOnly _returnvalue 0 "DoNotLock" false)
  (Game|SetGamePaused true))

(event Input|KeyboardEvents|DebugKey1
  (params (Key :type Key%20Structure :default "None") (ActionValue :type Input%20Action%20Value%20Structure))
  ;[1 1 1] Respawn
  (:Pressed
    (Game|Damage|ApplyDamage self 1.0 0 0)))

(event Input|KeyboardEvents|DebugKeyP
  (params (Key :type Key%20Structure :default "None") (ActionValue :type Input%20Action%20Value%20Structure))
  ;[1 1 1] Pause Menu?
)

(fn ConstructionScript)