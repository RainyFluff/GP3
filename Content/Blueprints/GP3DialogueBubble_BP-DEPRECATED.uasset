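; Deprecated dialogue bubble Blueprint that displays a configurable line of text.
; On BeginPlay it converts the DisplayText variable to text and applies it to the Text component.
; ActivateText and DeactivateText events show and hide that component without propagating visibility to its children.
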(event `self.ReceiveBeginPlay`
  (`TextRenderComponent.K2_SetText` (`self.Text`) (`KismetTextLibrary.Conv_StringToText` (`self.DisplayText`))))

(event `self.ActivateText`
  (`SceneComponent.SetVisibility` (`self.Text`) (`self.true`) false))

(event `self.DeactivateText`
  (`SceneComponent.SetVisibility` (`self.Text`) (`self.false`) false))

(fn `UserConstructionScript`)