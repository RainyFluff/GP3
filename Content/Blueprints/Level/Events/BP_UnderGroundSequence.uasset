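; BP_UnderGroundSequence is a one-shot level event in which a hidden wooden-spoon mesh, acting as a knife, stabs downward.
; An overlap on Collider reveals the spoon, and if the main character triggered it, a timeline lerps the mesh down by StabDepth and plays a strike sound once.
; A separate WeaponCollider destroys overlapping actors tagged Killable and fires a Niagara cookie-death effect at their location.
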(event `self.ReceiveBeginPlay`
  ;[1 1 1] "Constructor"
  (`SceneComponent.SetVisibility` (`self.SM_wood_spoon`) false false))

(event `self.Collider.OnComponentBeginOverlap`
  (params (OverlappedComponent :type "PrimitiveComponent Object Reference") (OtherActor :type "Actor Object Reference") (OtherComp :type "PrimitiveComponent Object Reference") (OtherBodyIndex :type Integer) (bFromSweep :type Boolean) (SweepResult :type "HitResult Structure (by ref)"))
  (bind _sm_wood_spoon (`self.SM_wood_spoon`))
  (bind _returnvalue (`SceneComponent.K2_GetComponentLocation` _sm_wood_spoon))
  ;[1 1 1] Animating the knife
  (if (`self.CanTrigger`)
    (`|ExecutionSequence`
      (:`then_0`
        (bind _output_get (set `self.StabPos` _returnvalue)))
      (:`then_1`
        (cast `/Game/Blueprints/Player/BP_MainCharacter` OtherActor
          (:`then`
            (set `self.CanTrigger` false)
            (bind (_direction _percentage) (`Timeline|Anim`)
              (:`Update`
                (`SceneComponent.K2_SetWorldLocation` _sm_wood_spoon (`KismetMathLibrary.VLerp` _returnvalue (- _output_get (`KismetMathLibrary.MakeVector` 0.0 0.0 (`self.StabDepth`))) _percentage) false false)
                (`/Engine/EditorBlueprintResources/StandardMacros.DoOnce` false
                  (:`Completed`
                    (bind _returnvalue_2 (`GameplayStatics.SpawnSound2D` "/Game/Audio/KnifeStrike1.KnifeStrike1" 1.0 1.0 0.0 null))
                    (set `self.KnifeSound` _returnvalue_2))))))
          (:`CastFailed`
            (`KismetSystemLibrary.PrintString` "Failed Cast"))))
      (:`then_2`
        (`SceneComponent.SetVisibility` (`self.SM_wood_spoon`) true false)))))

(event `self.WeaponCollider.OnComponentBeginOverlap`
  (params (OverlappedComponent :type "PrimitiveComponent Object Reference") (OtherActor :type "Actor Object Reference") (OtherComp :type "PrimitiveComponent Object Reference") (OtherBodyIndex :type Integer) (bFromSweep :type Boolean) (SweepResult :type "HitResult Structure (by ref)"))
  (bind _fx_ng_cookiedeath (`self.FX_NG_CookieDeath`))
  ;[1 1 1] Destroying the "npc's" it collides with
  (if (`self.ActorHasTag` OtherActor "Killable")
    (`SceneComponent.K2_SetWorldLocation` _fx_ng_cookiedeath (`self.K2_GetActorLocation` OtherActor) false false)
    (`self.K2_DestroyActor` OtherActor)
    (`ActorComponent.Activate` _fx_ng_cookiedeath false)))

(fn `UserConstructionScript`)