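; BP_MovableObject is a level object that the main character can push, flagging the character as pushing while it moves.
; X and Y colliders track when BP_MainCharacter overlaps and clear its IsPushingObj flag on exit.
; While overlapping, Tick sets that flag from whether the mesh velocity exceeds a small threshold.
; A separate collision sphere toggles the mesh's custom depth for a post-process shader when the character is near.
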(event `self.ReceiveTick`
  (params (DeltaSeconds :type "Float (single-precision)"))
  ;[1 1 1] Updating check if player is pushing Movable Object
  (if (`self.IsOverlapping`)
    (`/Engine/EditorBlueprintResources/StandardMacros.IsValid` (`self.MainCharacter`)
      (:`Is Valid`
        (bind _output_get (set `self.isMoving` (> (`KismetMathLibrary.VSize` (`SceneComponent.GetComponentVelocity` (`self.Mesh`))) 10.0)))
        (set `/Game/Blueprints/Player/BP_MainCharacter.IsPushingObj` _output_get (`self.MainCharacter`))))))

(event `self.XCollider.OnComponentBeginOverlap`
  (params (OverlappedComponent :type "PrimitiveComponent Object Reference") (OtherActor :type "Actor Object Reference") (OtherComp :type "PrimitiveComponent Object Reference") (OtherBodyIndex :type Integer) (bFromSweep :type Boolean) (SweepResult :type "HitResult Structure (by ref)"))
  ;[1 1 1] On overlap x Collider
  (bind _asbp_main_character (cast `/Game/Blueprints/Player/BP_MainCharacter` OtherActor))
  (set `self.MainCharacter` _asbp_main_character)
  (set `self.IsOverlapping` true))

(event `self.XCollider.OnComponentEndOverlap`
  (params (OverlappedComponent :type "PrimitiveComponent Object Reference") (OtherActor :type "Actor Object Reference") (OtherComp :type "PrimitiveComponent Object Reference") (OtherBodyIndex :type Integer))
  ;[1 1 1] On overlap x Collider
  (bind _asbp_main_character (cast `/Game/Blueprints/Player/BP_MainCharacter` OtherActor))
  (set `self.IsOverlapping` false)
  (set `/Game/Blueprints/Player/BP_MainCharacter.IsPushingObj` false _asbp_main_character))

(event `self.YCollider.OnComponentBeginOverlap`
  (params (OverlappedComponent :type "PrimitiveComponent Object Reference") (OtherActor :type "Actor Object Reference") (OtherComp :type "PrimitiveComponent Object Reference") (OtherBodyIndex :type Integer) (bFromSweep :type Boolean) (SweepResult :type "HitResult Structure (by ref)"))
  ;[1 1 1] On overlap Y collider
  (bind _asbp_main_character (cast `/Game/Blueprints/Player/BP_MainCharacter` OtherActor))
  (set `self.MainCharacter` _asbp_main_character)
  (set `self.IsOverlapping` true))

(event `self.YCollider.OnComponentEndOverlap`
  (params (OverlappedComponent :type "PrimitiveComponent Object Reference") (OtherActor :type "Actor Object Reference") (OtherComp :type "PrimitiveComponent Object Reference") (OtherBodyIndex :type Integer))
  ;[1 1 1] On overlap Y collider
  (bind _asbp_main_character (cast `/Game/Blueprints/Player/BP_MainCharacter` OtherActor))
  (set `self.IsOverlapping` false)
  (set `/Game/Blueprints/Player/BP_MainCharacter.IsPushingObj` false _asbp_main_character))

(event `self.CollisionSphere.OnComponentBeginOverlap`
  (params (OverlappedComponent :type "PrimitiveComponent Object Reference") (OtherActor :type "Actor Object Reference") (OtherComp :type "PrimitiveComponent Object Reference") (OtherBodyIndex :type Integer) (bFromSweep :type Boolean) (SweepResult :type "HitResult Structure (by ref)"))
  ;[1 1 1] Set render depth true/false for post process shader
  (cast `/Game/Blueprints/Player/BP_MainCharacter` OtherActor)
  (`PrimitiveComponent.SetRenderCustomDepth` (`self.Mesh`) true))

(event `self.CollisionSphere.OnComponentEndOverlap`
  (params (OverlappedComponent :type "PrimitiveComponent Object Reference") (OtherActor :type "Actor Object Reference") (OtherComp :type "PrimitiveComponent Object Reference") (OtherBodyIndex :type Integer))
  ;[1 1 1] Set render depth true/false for post process shader
  (cast `/Game/Blueprints/Player/BP_MainCharacter` OtherActor)
  (`PrimitiveComponent.SetRenderCustomDepth` (`self.Mesh`) false))

(fn `UserConstructionScript`)